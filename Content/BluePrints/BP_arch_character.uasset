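; BP_arch_character is a player character, apparently for architectural walkthroughs, with drag-to-look and drag-to-move mouse controls.
; Tick runs two gates: holding left mouse opens camera pitch/yaw rotation via RotateCam and shows a closed-hand cursor.
; Holding right mouse opens movement along the actor's forward and right vectors from raw axis key values.
; Forward and Right axis inputs also move the character directly.
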(event `self.ReceiveTick`
  (params (DeltaSeconds :type "Float (single-precision)"))
  ;[1 1 1] Camera Rotation with Mouse
  (`|ExecutionSequence`
    (:`then_0`
      (`/Engine/EditorBlueprintResources/StandardMacros.Gate` true :!label _label
        (:`Exit`
          (`self.RotateCam`))))
    (:`then_1`
      (`/Engine/EditorBlueprintResources/StandardMacros.Gate` true :!label _label_2
        (:`Exit`
          (`|ExecutionSequence`
            (:`then_0`
              (`self.AddMovementInput` (`self.GetActorForwardVector`) (`self.GetInputAxisKeyValue`)))
            (:`then_1`
              (`self.AddMovementInput` (`self.GetActorRightVector`) (* (`self.GetInputAxisKeyValue`) -1.0)))))))))

(event `Key|LeftMouseButton`
  (params (Key :type "Key Structure"))
  ;[1 1 1] Camera Rotation with Mouse
  (:`Pressed`
    (`self.grabCursor`)
    (goto _label :!via `Open`))
  (:`Released`
    (`self.defaultCursor`)
    (goto _label :!via `Close`)))

(event `Key|RightMouseButton`
  (params (Key :type "Key Structure"))
  (:`Pressed`
    (goto _label_2 :!via `Open`))
  (:`Released`
    (goto _label_2 :!via `Close`)))

(event `InputAxis|Forward`
  (params (AxisValue :type "Float (single-precision)"))
  ;[1 1 1] Moving the Character
  (`self.AddMovementInput` (`self.GetActorForwardVector`) AxisValue))

(event `InputAxis|Right`
  (params (AxisValue :type "Float (single-precision)"))
  ;[1 1 1] Moving the Character
  (`self.AddMovementInput` (`self.GetActorRightVector`) AxisValue))

(fn `defaultCursor`
  (set `PlayerController.CurrentMouseCursor` "Default" (`GameplayStatics.GetPlayerController` 0))
  (return))

(fn `grabCursor`
  (set `PlayerController.CurrentMouseCursor` "GrabHandClosed" (`GameplayStatics.GetPlayerController` 0))
  (return))

(fn `RotateCam`
  (`|ExecutionSequence`
    (:`then_0`
      (`self.AddControllerPitchInput` (* (`self.GetInputAxisKeyValue`) -1.0)))
    (:`then_1`
      (`self.AddControllerYawInput` (* (`self.GetInputAxisKeyValue`) 1.0)))))

(fn `UserConstructionScript`)